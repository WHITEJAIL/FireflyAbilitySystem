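; BP_PlayerCharacter is the player character, handling movement, camera look and melee combat through the Firefly ability system.
; BeginPlay links the combat anim layer, adds the input mapping and grants light and large attack combo chains plus a power attack, bound to Enhanced Input actions.
; Axis inputs move relative to control yaw, and Tab toggles between controller-facing and movement-facing rotation.
; Holding defense adds an InDefense tag until release.
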(event `self.ReceiveBeginPlay`
  (`SkeletalMeshComponent.LinkAnimClassLayers` (`self.Mesh`) "/FireflyAbilitySystem/Characters/Mannequin/Animations/Blueprints/ABP_Mannequin_StateLayer_Combat.ABP_Mannequin_StateLayer_Combat_C")
  (`EnhancedInputSubsystemInterface.AddMappingContext` (pcsubsystem `EnhancedInputLocalPlayerSubsystem` (`GameplayStatics.GetPlayerController` 0)) "/FireflyAbilitySystem/Blueprints/Input/IMC_Sample.IMC_Sample" 0 (struct))
  (`|ExecutionSequence`
    (:`then_0`
      (`FireflyAbilityManagerComponent.GrantAbility` (`self.FireflyPlayerAbilityManager`) "/FireflyAbilitySystem/Blueprints/Ability/Combo1/FA_Combo1_1.FA_Combo1_1_C")
      (`FireflyPlayerAbilityManagerComponent.BindAbilityToInput` (`self.FireflyPlayerAbilityManager`) "/FireflyAbilitySystem/Blueprints/Ability/Combo1/FA_Combo1_1.FA_Combo1_1_C" "/FireflyAbilitySystem/Blueprints/Input/IA_LightAtk.IA_LightAtk")
      (`FireflyAbilityManagerComponent.GrantAbility` (`self.FireflyPlayerAbilityManager`) "/FireflyAbilitySystem/Blueprints/Ability/Combo1/FA_Combo1_2.FA_Combo1_2_C")
      (`FireflyPlayerAbilityManagerComponent.BindAbilityToInput` (`self.FireflyPlayerAbilityManager`) "/FireflyAbilitySystem/Blueprints/Ability/Combo1/FA_Combo1_2.FA_Combo1_2_C" "/FireflyAbilitySystem/Blueprints/Input/IA_LightAtk.IA_LightAtk")
      (`FireflyAbilityManagerComponent.GrantAbility` (`self.FireflyPlayerAbilityManager`) "/FireflyAbilitySystem/Blueprints/Ability/Combo1/FA_Combo1_3.FA_Combo1_3_C")
      (`FireflyPlayerAbilityManagerComponent.BindAbilityToInput` (`self.FireflyPlayerAbilityManager`) "/FireflyAbilitySystem/Blueprints/Ability/Combo1/FA_Combo1_3.FA_Combo1_3_C" "/FireflyAbilitySystem/Blueprints/Input/IA_LightAtk.IA_LightAtk")
      (`FireflyAbilityManagerComponent.GrantAbility` (`self.FireflyPlayerAbilityManager`) "/FireflyAbilitySystem/Blueprints/Ability/Combo1/FA_Combo1_4.FA_Combo1_4_C")
      (`FireflyPlayerAbilityManagerComponent.BindAbilityToInput` (`self.FireflyPlayerAbilityManager`) "/FireflyAbilitySystem/Blueprints/Ability/Combo1/FA_Combo1_4.FA_Combo1_4_C" "/FireflyAbilitySystem/Blueprints/Input/IA_LightAtk.IA_LightAtk"))
    (:`then_1`
      (`FireflyAbilityManagerComponent.GrantAbility` (`self.FireflyPlayerAbilityManager`) "/FireflyAbilitySystem/Blueprints/Ability/Combo2/FA_Combo2_1.FA_Combo2_1_C")
      (`FireflyPlayerAbilityManagerComponent.BindAbilityToInput` (`self.FireflyPlayerAbilityManager`) "/FireflyAbilitySystem/Blueprints/Ability/Combo2/FA_Combo2_1.FA_Combo2_1_C" "/FireflyAbilitySystem/Blueprints/Input/IA_LargeAtk.IA_LargeAtk")
      (`FireflyAbilityManagerComponent.GrantAbility` (`self.FireflyPlayerAbilityManager`) "/FireflyAbilitySystem/Blueprints/Ability/Combo2/FA_Combo2_2.FA_Combo2_2_C")
      (`FireflyPlayerAbilityManagerComponent.BindAbilityToInput` (`self.FireflyPlayerAbilityManager`) "/FireflyAbilitySystem/Blueprints/Ability/Combo2/FA_Combo2_2.FA_Combo2_2_C" "/FireflyAbilitySystem/Blueprints/Input/IA_LargeAtk.IA_LargeAtk")
      (`FireflyAbilityManagerComponent.GrantAbility` (`self.FireflyPlayerAbilityManager`) "/FireflyAbilitySystem/Blueprints/Ability/Combo2/FA_Combo2_3.FA_Combo2_3_C")
      (`FireflyPlayerAbilityManagerComponent.BindAbilityToInput` (`self.FireflyPlayerAbilityManager`) "/FireflyAbilitySystem/Blueprints/Ability/Combo2/FA_Combo2_3.FA_Combo2_3_C" "/FireflyAbilitySystem/Blueprints/Input/IA_LargeAtk.IA_LargeAtk")
      (`FireflyAbilityManagerComponent.GrantAbility` (`self.FireflyPlayerAbilityManager`) "/FireflyAbilitySystem/Blueprints/Ability/Combo2/FA_Combo2_4.FA_Combo2_4_C")
      (`FireflyPlayerAbilityManagerComponent.BindAbilityToInput` (`self.FireflyPlayerAbilityManager`) "/FireflyAbilitySystem/Blueprints/Ability/Combo2/FA_Combo2_4.FA_Combo2_4_C" "/FireflyAbilitySystem/Blueprints/Input/IA_LargeAtk.IA_LargeAtk"))
    (:`then_2`
      (`FireflyAbilityManagerComponent.GrantAbility` (`self.FireflyPlayerAbilityManager`) "/FireflyAbilitySystem/Blueprints/Ability/Common/FA_PowerAttack.FA_PowerAttack_C")
      (`FireflyPlayerAbilityManagerComponent.BindAbilityToInput` (`self.FireflyPlayerAbilityManager`) "/FireflyAbilitySystem/Blueprints/Ability/Common/FA_PowerAttack.FA_PowerAttack_C" "/FireflyAbilitySystem/Blueprints/Input/IA_LightAtk.IA_LightAtk"))))

(event `InputAxis|Forward`
  (params (AxisValue :type "Float (single-precision)"))
  (`self.AddMovementInput` (`KismetMathLibrary.GetForwardVector` (`KismetMathLibrary.MakeRotator` 0.0 0.0 (.yaw (`self.GetControlRotation`)))) AxisValue))

(event `InputAxis|Right`
  (params (AxisValue :type "Float (single-precision)"))
  (`self.AddMovementInput` (`KismetMathLibrary.GetRightVector` (`KismetMathLibrary.MakeRotator` 0.0 0.0 (.yaw (`self.GetControlRotation`)))) AxisValue))

(event `InputAxis|Turn`
  (params (AxisValue :type "Float (single-precision)"))
  (`self.AddControllerYawInput` AxisValue))

(event `InputAxis|LookUp`
  (params (AxisValue :type "Float (single-precision)"))
  (`self.AddControllerPitchInput` AxisValue))

(event `Key|Tab`
  (params (Key :type "Key Structure"))
  (bind _charactermovement (`self.CharacterMovement`))
  (:`Pressed`
    (`/Engine/EditorBlueprintResources/StandardMacros.FlipFlop`
      (:`A`
        (set `self.bUseControllerRotationYaw` true)
        (set `CharacterMovementComponent.bOrientRotationToMovement` false _charactermovement))
      (:`B`
        (set `self.bUseControllerRotationYaw` false)
        (set `CharacterMovementComponent.bOrientRotationToMovement` true _charactermovement)))))

(event `EnhancedInput|/FireflyAbilitySystem/Blueprints/Input/IA_Defense`
  (params (ActionValue :type Boolean) (ElapsedSeconds :type "Float (double-precision)") (TriggeredSeconds :type "Float (double-precision)") (InputAction :type "InputAction Object Reference" :default "/FireflyAbilitySystem/Blueprints/Input/IA_Defense.IA_Defense"))
  (bind _fireflytagmanager (`self.FireflyTagManager`))
  (:`Started`
    (`FireflyTagManagerComponent.AddTagToManager` _fireflytagmanager (struct :`TagName` "AbilityState.InDefense") 1))
  (:`Completed`
    (`FireflyTagManagerComponent.RemoveTagFromManager` _fireflytagmanager (struct :`TagName` "AbilityState.InDefense") 1)))

(fn `UserConstructionScript`)