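; ANS_ContainTag is an anim notify state that grants a configurable gameplay tag to the animating actor for the duration of the notify window.
; On begin it adds one count of TagToContain to the owner's FireflyAbilitySystemComponent tag manager, and on end it removes one count.
; The notify's display name is the tag's debug string.
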(fn `GetNotifyName`
  (returns (ReturnValue :type String))
  (return (`BlueprintGameplayTagLibrary.GetDebugStringFromGameplayTag` (`self.TagToContain`))))

(fn `Received_NotifyBegin`
  (params (MeshComp :type "SkeletalMeshComponent Object Reference") (Animation :type "AnimSequenceBase Object Reference") (TotalDuration :type "Float (single-precision)") (EventReference :type "AnimNotifyEventReference Structure (by ref)"))
  (returns (ReturnValue :type Boolean))
  (`FireflyAbilitySystemComponent.AddTagToManager` (`Actor.GetComponentByClass` (`ActorComponent.GetOwner` MeshComp) "/Script/FireflyAbilitySystem.FireflyAbilitySystemComponent") (`self.TagToContain`) 1)
  (return true))

(fn `Received_NotifyEnd`
  (params (MeshComp :type "SkeletalMeshComponent Object Reference") (Animation :type "AnimSequenceBase Object Reference") (EventReference :type "AnimNotifyEventReference Structure (by ref)"))
  (returns (ReturnValue :type Boolean))
  (`FireflyAbilitySystemComponent.RemoveTagFromManager` (`Actor.GetComponentByClass` (`ActorComponent.GetOwner` MeshComp) "/Script/FireflyAbilitySystem.FireflyAbilitySystemComponent") (`self.TagToContain`) 1)
  (return true))