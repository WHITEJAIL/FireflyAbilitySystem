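; FA_Sample is a sample combo attack ability that plays one section of AM_Combo_Attack_01 on the owning Character's mesh per activation.
; The section name is the Index counter converted to a name.
; Completed, Blend Out and Interrupted all increment Index and wrap it to zero past 3, so one playback can advance it more than once.
; The graph has no explicit end-ability call.
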(event `self.ReceiveActivateAbility`
  (bind _ascharacter (cast `Character` (`self.GetOwnerActor`)))
  (`|PlayMontage` (`Character.Mesh` _ascharacter) "/FireflyAbilitySystem/Characters/Mannequin/Animations/Sequence/02_Attack/01_Combo_Attack_01/AM_Combo_Attack_01.AM_Combo_Attack_01" 1.0 0.0 (`KismetStringLibrary.Conv_StringToName` (`KismetStringLibrary.Conv_IntToString` (`self.Index`)))
    (:`OnCompleted`
      _)
    (:`OnBlendOut`
      _)
    (:`OnInterrupted`
      _))
  (bind _result (`/Engine/EditorBlueprintResources/StandardMacros.IncrementInt` (`self.Index`))
    (:`  `
      (if (> _result 3)
        (set `self.Index` 0)))))